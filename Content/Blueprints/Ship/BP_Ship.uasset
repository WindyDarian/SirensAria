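; Networked player ship with wheel steering, left and right cannon batteries, health and a cannonball counter.
; Tick yaws the ship by wheel angle, eases the wheel back without input, moves forward and syncs the angle through server and multicast events.
; A looping server timer multicasts transform corrections to remotes.
; Child-actor cannons are gathered at BeginPlay for aiming and per-side cooldown firing, while damage is applied on authority.
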(event Custom|CorrectLocRot
  ;[1 1 1] Location Correction
  (CallFunction|MCCorrectLocRot (Transformation|GetActorRotation) (Transformation|GetActorLocation)))

(event Custom|FireLeft
  (if (not (Variables|Default|GetbLeftOnCooldown))
    (CallFunction|MCFireLeft)))

(event Custom|FireRight
  (if (not (Variables|Default|GetbRightOnCooldown))
    (CallFunction|MCFireRight)))

(event Custom|CDLeft
  (Variables|Default|SetbLeftOnCooldown false))

(event Custom|CDRight
  (Variables|Default|SetbRightOnCooldown false))

(event Custom|CannonRight
  (params (axis_value :type Float%20%28single-precision%29))
  (Class|Cannon|RotateRight (Variables|Default|GetLeftCannons) axis_value)
  (Class|Cannon|RotateRight (Variables|Default|GetRightCannons) axis_value))

(event Custom|MCFireLeft
  (Class|Cannon|Fire (Variables|Default|GetLeftCannons))
  (Variables|Default|SetbLeftOnCooldown true)
  (Utilities|Time|SetTimerbyEvent (delegate Custom|CDLeft) (Variables|Default|Getfire_cooldown)))

(event Custom|MCFireRight
  (Class|Cannon|Fire (Variables|Default|GetRightCannons))
  (Variables|Default|SetbRightOnCooldown true)
  (Utilities|Time|SetTimerbyEvent (delegate Custom|CDRight) (Variables|Default|Getfire_cooldown)))

(event Custom|CannonUp
  (params (axis_value :type Float%20%28single-precision%29))
  (Class|Cannon|RotateUp (Variables|Default|GetLeftCannons) axis_value)
  (Class|Cannon|RotateUp (Variables|Default|GetRightCannons) axis_value))

(event Custom|ServerSyncWheelRot
  (params (WheelRot :type Float%20%28single-precision%29))
  (bind _output_get (Variables|Default|SetWheelRotationX WheelRot))
  (CallFunction|MCWheelRot _output_get))

(event Custom|MCWheelRot
  (params (wheel_rot :type Float%20%28single-precision%29))
  (if (!= (Components|GetOwner) (Game|GetPlayerController 0))
    (Variables|Default|SetWheelRotationX wheel_rot)))

(event Custom|MC_CorrectLocRot
  (params (Server_Rotation :type Rotator) (Server_Location :type Vector))
  (Networking|SwitchHasAuthority
    (:Remote
      (Transformation|SetActorLocationAndRotation Server_Location Server_Rotation true))))

(event EventBeginPlay
  (Utilities|FlowControl|Sequence
    (:then_0
      (Utilities|FlowControl|Sequence
        (:then_0
          ;[1 1 1] Add Cannons
          (Utilities|FlowControl|Sequence
            (:then_0
              (for _array_element (Components|GetChildrenComponents (Variables|Default|GetLeftCannonArrow) false)
                (bind _aschild_actor_component (Utilities|Casting|CastToChildActorComponent _array_element))
                (bind _ascannon (Utilities|Casting|CastToCannon (Variables|/Script/Engine.ChildActorComponent|GetChildActor _aschild_actor_component)))
                (Utilities|Array|AddUnique (Variables|Default|GetLeftCannons) _ascannon)
                (Actor|SetOwner _ascannon self)))
            (:then_1
              (for _array_element_2 (Components|GetChildrenComponents (Variables|Default|GetRightCannonArrow) false)
                (bind _aschild_actor_component_2 (Utilities|Casting|CastToChildActorComponent _array_element_2))
                (bind _ascannon_2 (Utilities|Casting|CastToCannon (Variables|/Script/Engine.ChildActorComponent|GetChildActor _aschild_actor_component_2)))
                (Utilities|Array|AddUnique (Variables|Default|GetRightCannons) _ascannon_2)
                (Actor|SetOwner _ascannon_2 self)))))
        (:then_1
          ;[1 1 1] Location Correction
          (Networking|SwitchHasAuthority
            (:Authority
              (Utilities|Time|SetTimerbyEvent (delegate Custom|CorrectLocRot) 3.0 true))))))
    (:then_1
      (bind _ashealth_bars (Utilities|Casting|CastToHealthBars (UserInterface|GetUserWidgetObject (Variables|Default|GetWidget))))
      (Variables|/Game/Blueprints/Widgets/HealthBars.HealthBars_C|Setowner_ship _ashealth_bars self))))

(event EventActorBeginOverlap
  (params (OtherActor :type Actor%20Object%20Reference)))

(event EventTick
  (params (DeltaSeconds :type Float%20%28single-precision%29))
  (bind _returnvalue (Transformation|GetActorRotation))
  (bind _wheel (Variables|Default|GetWheel))
  (bind (_roll _pitch _yaw) (Math|Rotator|BreakRotator _returnvalue))
  (bind _relativerotation (Variables|/Script/Engine.SceneComponent|GetRelativeRotation _wheel))
  (bind (_roll_2 _pitch_2 _yaw_2) (Math|Rotator|BreakRotator _relativerotation))
  (Utilities|FlowControl|Sequence
    (:then_0
      (Utilities|FlowControl|Sequence
        (:then_0
          ;[1 1 1] Steer ship by wheel rotation
          (Transformation|SetActorRotation (Math|Rotator|MakeRotator _roll _pitch (+ (* (Variables|Default|GetWheelRotationX) DeltaSeconds 0.05) _yaw))))
        (:then_1
          ;[1 1 1] TODO: Return Wheel
          (if (Variables|Default|GetbWheelInputSet)
            (Variables|Default|SetbWheelInputSet false)
            (else
              (Variables|Default|SetWheelRotationX (* (Variables|Default|GetWheelRotationX) (- 1.0 (* (Variables|Default|GetWheelReturnRate) DeltaSeconds)))))))
        (:then_2
          ;[1 1 1] Set Wheel Rotation
          (Transformation|SetRelativeRotation _wheel (Math|Rotator|MakeRotator (Variables|Default|GetWheelRotationX) _pitch_2 _yaw_2) false false))
        (:then_3
          ;[1 1 1] TEMP: moving forward
          (Transformation|AddActorLocalOffset (Math|Vector|MakeVector (* (Variables|Default|Getspeed) DeltaSeconds) 0.0 0.0) true false))
        (:then_4
          (CallFunction|ServerSyncWheelRot (Variables|Default|GetWheelRotationX)))))))

(event Game|Damage|EventAnyDamage
  (params (Damage :type Float%20%28single-precision%29) (DamageType :type Damage%20Type%20Object%20Reference) (InstigatedBy :type Controller%20Object%20Reference) (DamageCauser :type Actor%20Object%20Reference))
  (Networking|SwitchHasAuthority
    (:Authority
      (CallFunction|ReceiveDamage Damage))))

(fn ConstructionScript)

(fn SetWheelInput
  (params (rotateX :type Float%20%28single-precision%29))
  (if (> (Math|Float|Absolute(Float) rotateX) 0.05)
    (Variables|Default|SetbWheelInputSet true)
    (Variables|Default|SetWheelRotationX (Math|Float|Clamp(Float) (+ rotateX (Variables|Default|GetWheelRotationX)) (Variables|Default|Getwheel_range_min) (Variables|Default|Getwheel_range_max)))))

(fn AttachPlayerCharacter
  (params (character :type Leap%20My%20Character%20Object%20Reference))
  (Class|Actor|AttachRootComponentto character (Variables|Default|GetPlayerLocator) "None" "SnapToTarget" true)
  (Variables|/Game/Blueprints/LeapMyCharacter.LeapMyCharacter_C|SetBP_Ship character self)
  (Variables|Default|Setcharacter character))

(fn ReceiveDamage
  (params (amount :type Float%20%28single-precision%29))
  (Variables|Default|Sethealth (Math|Float|Clamp(Float) (- (Variables|Default|Gethealth) amount) 0.0 (Variables|Default|Getmax_health))))

(fn GetShipVelocity
  (return (* (Math|Vector|GetForwardVector (Transformation|GetActorRotation self)) (Variables|Default|Getspeed))))

(fn GetHealthPercentage
  (return (Math|Float|Clamp(Float) (/ (Variables|Default|Gethealth) (Variables|Default|Getmax_health)))))

(fn SetWheelRotation
  (params (rotationX :type Float%20%28single-precision%29))
  (Variables|Default|SetbWheelInputSet true)
  (Variables|Default|SetWheelRotationX (Math|Float|Clamp(Float) rotationX (Variables|Default|Getwheel_range_min) (Variables|Default|Getwheel_range_max))))

(fn PickUpCannonball
  (Variables|Default|Settotal_cannonball (+ (Variables|Default|Gettotal_cannonball) 1)))

(fn GetTotalCannonball
  (return (Variables|Default|Gettotal_cannonball)))