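; Player ship with a steering wheel and port and starboard cannon batteries, gathered from child actors at BeginPlay.
; Wheel input accumulates into a rotation that, on authority, sets yaw rate, eases back when idle and turns the wheel mesh, alongside temporary constant forward movement.
; Non-authority instances send their wheel rotation through ServerSyncWheelRot every tick.
; Each battery fires behind its own timer cooldown, and characters attach at PlayerLocator.
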(event Custom|CDLeft
  (Variables|Default|SetbLeftOnCooldown false))

(event Custom|CDRight
  (Variables|Default|SetbRightOnCooldown false))

(event Custom|ServerSyncWheelRot
  (params (WheelRot :type Float%20%28single-precision%29))
  (Variables|Default|SetWheelRotationX WheelRot))

(event Custom|FireLeft
  (bind _leftcannons (Variables|Default|GetLeftCannons))
  (if (not (Variables|Default|GetbLeftOnCooldown))
    (for _array_element _leftcannons
      (Class|Cannon|Fire _leftcannons)
      (Variables|Default|SetbLeftOnCooldown true)
      (Utilities|Time|SetTimerbyEvent (delegate Custom|CDLeft) (Variables|Default|Getfire_cooldown)))))

(event Custom|FireRight
  (bind _rightcannons (Variables|Default|GetRightCannons))
  (if (not (Variables|Default|GetbRightOnCooldown))
    (for _array_element _rightcannons
      (Class|Cannon|Fire _rightcannons)
      (Variables|Default|SetbRightOnCooldown true)
      (Utilities|Time|SetTimerbyEvent (delegate Custom|CDRight) (Variables|Default|Getfire_cooldown)))))

(event EventBeginPlay
  ;[1 1 1] Add Cannons
  (Utilities|FlowControl|Sequence
    (:then_0
      (for _array_element (Components|GetChildrenComponents (Variables|Default|GetLeftCannonArrow) false)
        (bind _aschild_actor_component (Utilities|Casting|CastToChildActorComponent _array_element))
        (bind _ascannon (Utilities|Casting|CastToCannon (Variables|/Script/Engine.ChildActorComponent|GetChildActor _aschild_actor_component)))
        (Utilities|Array|AddUnique (Variables|Default|GetLeftCannons) _ascannon)))
    (:then_1
      (for _array_element_2 (Components|GetChildrenComponents (Variables|Default|GetRightCannonArrow) false)
        (bind _aschild_actor_component_2 (Utilities|Casting|CastToChildActorComponent _array_element_2))
        (bind _ascannon_2 (Utilities|Casting|CastToCannon (Variables|/Script/Engine.ChildActorComponent|GetChildActor _aschild_actor_component_2)))
        (Utilities|Array|AddUnique (Variables|Default|GetRightCannons) _ascannon_2)))))

(event Collision|EventActorBeginOverlap
  (params (OtherActor :type Actor%20Object%20Reference)))

(event EventTick
  (params (DeltaSeconds :type Float%20%28single-precision%29))
  (bind _returnvalue (Transformation|GetActorRotation))
  (bind _wheel (Variables|Default|GetWheel))
  (bind (_roll _pitch _yaw) (Math|Rotator|BreakRotator _returnvalue))
  (bind _relativerotation (Variables|/Script/Engine.SceneComponent|GetRelativeRotation _wheel))
  (bind (_roll_2 _pitch_2 _yaw_2) (Math|Rotator|BreakRotator _relativerotation))
  (Networking|SwitchHasAuthority
    (:Authority
      (Utilities|FlowControl|Sequence
        (:then_0
          ;[1 1 1] Steer ship by wheel rotation
          (Transformation|SetActorRotation (Math|Rotator|MakeRotator _roll _pitch (+ (* (Variables|Default|GetWheelRotationX) DeltaSeconds 0.25) _yaw))))
        (:then_1
          (if (Variables|Default|GetbWheelInputSet)
            (Variables|Default|SetbWheelInputSet false)
            (else
              (Variables|Default|SetWheelRotationX (* (Variables|Default|GetWheelRotationX) (- 1.0 (* (Variables|Default|GetWheelReturnRate) DeltaSeconds)))))))
        (:then_2
          ;[1 1 1] Set Wheel Rotation
          (Transformation|SetRelativeRotation _wheel (Math|Rotator|MakeRotator (Variables|Default|GetWheelRotationX) _pitch_2 _yaw_2) false false))
        (:then_3
          ;[1 1 1] TEMP: moving forward
          (Transformation|AddActorLocalOffset (Math|Vector|MakeVector (* (Variables|Default|Getspeed) DeltaSeconds) 0.0 0.0) true false))))
    (:Remote
      (CallFunction|ServerSyncWheelRot (Variables|Default|GetWheelRotationX)))))

(fn ConstructionScript)

(fn SetWheelInput
  (params (rotateX :type Float%20%28single-precision%29))
  (if true
    (if (> (Math|Float|Absolute(Float) rotateX) 0.05)
      (Variables|Default|SetbWheelInputSet true)
      (Variables|Default|SetWheelRotationX (+ rotateX (Variables|Default|GetWheelRotationX))))))

(fn AttachPlayerCharacter
  (params (character :type Leap%20My%20Character%20Object%20Reference))
  (Class|Actor|AttachRootComponentto character (Variables|Default|GetPlayerLocator) "None" "SnapToTarget" true)
  (Variables|/Game/Blueprints/LeapMyCharacter.LeapMyCharacter_C|SetBP_Ship character self)
  (Variables|Default|Setcharacter character))