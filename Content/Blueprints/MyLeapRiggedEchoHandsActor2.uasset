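; Leap Motion rigged hands actor that lets the player's hands touch BP_Ship actors, setting IsTouched on overlap begin and clearing it on end.
; Tick draws debug spheres at both middle-finger sockets and stores their positions, but moves LeftCollision to each in turn, leaving it on the right hand.
; ShowHand toggles each mesh's visibility, and Reconstruct, run from the construction script, sets both meshes' collision from EnablePhysicsCollision.
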(event EventReconstruct
  (bind _lefthandmesh (Variables|Default|GetLeftHandMesh))
  (if (Variables|Default|GetEnablePhysicsCollision)
    (Collision|SetCollisionEnabled _lefthandmesh "QueryAndPhysics")
    (else
      (Collision|SetCollisionEnabled _lefthandmesh "NoCollision"))))

(event Collision|EventActorBeginOverlap
  (params (OtherActor :type Actor%20Object%20Reference))
  ;[1 1 1] Comment
  (bind _asbp_ship (Utilities|Casting|CastToBP_Ship OtherActor))
  (Variables|/Game/Blueprints/Ship/BP_Ship.BP_Ship_C|SetisTouched _asbp_ship true))

(event Collision|EventActorEndOverlap
  (params (OtherActor :type Actor%20Object%20Reference))
  ;[1 1 1] Comment
  (bind _asbp_ship (Utilities|Casting|CastToBP_Ship OtherActor))
  (Variables|/Game/Blueprints/Ship/BP_Ship.BP_Ship_C|SetisTouched _asbp_ship false))

(event EventBeginPlay
  (|CallParentFunction))

(event Collision|EventActorBeginOverlap
  (params (OtherActor :type Actor%20Object%20Reference)))

(event EventShowHand
  (params (Hand :type LeapHandType%20Enum :default "HAND_UNKNOWN") (Visible :type Boolean))
  (bind _lefthandmesh (Variables|Default|GetLeftHandMesh))
  (bind _righthandmesh (Variables|Default|GetRightHandMesh))
  (switch Utilities|FlowControl|Switch|SwitchonLeapHandType Hand
    (:HAND_LEFT
      (if (Math|Boolean|NotEqual(Boolean) (Variables|/Script/Engine.SceneComponent|GetbVisible _lefthandmesh) Visible)
        (Rendering|SetVisibility _lefthandmesh Visible false)))
    (:HAND_RIGHT
      (if (Math|Boolean|NotEqual(Boolean) (Variables|/Script/Engine.SceneComponent|GetbVisible _righthandmesh) Visible)
        (Rendering|SetVisibility _righthandmesh Visible false)))))

(event EventTick
  (params (DeltaSeconds :type Float%20%28single-precision%29))
  (bind _lefthandmesh (Variables|Default|GetLeftHandMesh))
  (bind _righthandmesh (Variables|Default|GetRightHandMesh))
  (bind _returnvalue (Transformation|GetSocketLocation _lefthandmesh "lf_middle_a"))
  (bind _returnvalue_2 (Transformation|GetSocketLocation _righthandmesh "rt_middle_a"))
  ;[1 1 1] Move Collider
  (Rendering|Debug|DrawDebugSphere _returnvalue 5.0 12 "(R=1.000000,G=1.000000,B=1.000000,A=1.000000)" 0.0)
  (Transformation|SetWorldLocation (Variables|Default|GetLeftCollision) _returnvalue false false)
  (Variables|Default|SetleftHandPos _returnvalue)
  (Rendering|Debug|DrawDebugSphere _returnvalue_2 5.0 12 "(R=1.000000,G=1.000000,B=1.000000,A=1.000000)" 0.0)
  (Transformation|SetWorldLocation (Variables|Default|GetLeftCollision) _returnvalue_2 false false)
  (Variables|Default|SetrightHandPos _returnvalue_2))

(fn ConstructionScript
  (|CallParentFunction)
  (CallFunction|Reconstruct))

(fn GetSocketLocation
  (params (SocketName :type Name))
  (return (Transformation|GetSocketLocation (Variables|Default|GetLeftHandMesh) SocketName)))

(fn GetSocketRotation
  (params (Socket :type Name))
  (return (Transformation|GetSocketRotation (Variables|Default|GetLeftHandMesh) Socket)))